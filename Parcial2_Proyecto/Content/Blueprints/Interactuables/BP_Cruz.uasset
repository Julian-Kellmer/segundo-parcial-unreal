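; BP_Cruz is an interactable wall cross that the player rights, after which it turns itself upside down.
; EjecutarInteraccion disables further interaction and, if the interaction widget is valid, calls LevantarCruz; the widget removal node never runs.
; One timeline lerps the mesh to a raised position and upright rotation.
; After a delay, a second timeline rolls it 180 degrees.
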(event Custom|LevantarCruz
  (bind _rotacionlevantada (Variables|Cruz|GetRotacionLevantada))
  ;[0.15 0.15 0.15 0.5] levantar y enderezar
  (Variables|Cruz|SetPosicionInicial (Transformation|GetWorldLocation (Variables|Default|GetMeshCruz)))
  (Variables|Cruz|SetRotacionInicialCruz (Transformation|GetWorldRotation (Variables|Default|GetMeshCruz)))
  (bind _alpha (Timeline|TL_LevantarCruz PlayFromStart)
    (:Update
      (Transformation|SetWorldLocation (Variables|Default|GetMeshCruz) (Math|Vector|Lerp(Vector) (Variables|Cruz|GetPosicionInicial) (+ (Variables|Cruz|GetPosicionInicial) (Variables|Cruz|GetPosicionLevantada)) _alpha) false false)
      (Transformation|SetWorldRotation (Variables|Default|GetMeshCruz) (Math|Rotator|Lerp(Rotator) (Variables|Cruz|GetRotacionInicialCruz) (Variables|Cruz|GetRotacionLevantada) _alpha true) false false))
    (:Finished
      ;[0.15 0.15 0.15 0.5] invertir cruz
      (Utilities|FlowControl|Delay (Variables|Cruz|GetTiempoAntesDeInvertir))
      (bind _alpha_2 (Timeline|TL_InvertirCruz PlayFromStart)
        (:Update
          (Transformation|SetWorldRotation (Variables|Default|GetMeshCruz) (Math|Rotator|Lerp(Rotator) _rotacionlevantada (Math|Rotator|CombineRotators _rotacionlevantada (Math|Rotator|MakeRotator 1.8e+02 0.0 0.0)) _alpha_2) false false))))))

(fn ConstructionScript
  (|CallParentFunction))

(fn ObtenerTextoInteraccion
  (return "Presionà E para Acomodar la cruz en la pared"))

(fn EjecutarInteraccion
  (params (Instigador :type Actor%20Object%20Reference))
  (Variables|Default|SetbPuedeInteractuar false)
  (Utilities|IsValid (Variables|Default|GetWidgetInteraccion)
    (:Is%20Valid
      (CallFunction|LevantarCruz))))