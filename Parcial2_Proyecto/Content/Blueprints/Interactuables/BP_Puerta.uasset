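; Interactable door that swings open and closed when an instigator interacts with it.
; EjecutarInteraccion flips EstaAbierta and calls AnimarPuerta, which plays or reverses the TL_Puerta timeline.
; The timeline's alpha lerps the Bisagra hinge's relative yaw between zero and AnguloPuerta.
; ObtenerTextoInteraccion returns a Spanish press-E prompt to open or close, matching the current state.
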(event Custom|AnimarPuerta
  ;[0.15 0.15 0.15 0.5] Animacion apertura
  (if (Variables|Puerta|GetbEstaAbierta)
    (bind _alpha (Timeline|TL_Puerta Play)
      (:Update
        (Transformation|SetRelativeRotation (Variables|Default|GetBisagra) (Math|Rotator|MakeRotator 0.0 0.0 (Math|Float|Lerp 0.0 (Variables|Puerta|GetAnguloPuerta) _alpha)) false false)))
    (else
      (Timeline|TL_Puerta Reverse))))

(fn ConstructionScript
  (|CallParentFunction))

(fn EjecutarInteraccion
  (params (Instigador :type Actor%20Object%20Reference))
  (Variables|Puerta|SetbEstaAbierta (not (Variables|Puerta|GetbEstaAbierta)))
  (CallFunction|AnimarPuerta))

(fn ObtenerTextoInteraccion
  (return (select (Variables|Puerta|GetbEstaAbierta) "Presioná E para cerrar la puerta" "Presioná E para abrir la puerta")))