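; A locker prop that rattles and plays a shaking sound when a referenced door is interacted with.
; It binds to the observed door's interaction event at BeginPlay and caches the mesh's starting rotation.
; On trigger, a fast looping timer applies random roll and yaw offsets around that rotation, and a second timer stops the shake after a set duration and restores it.
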(event Custom|AlAbrirsePuerta
  (params (ActorInteractuado :type Actor%20Object%20Reference) (Instigador :type Actor%20Object%20Reference))
  (Audio|PlaySoundatLocation (Variables|Locker|GetSonidoTemblor) (Transformation|GetWorldLocation (Variables|Default|GetMeshLocker)) "0, 0, 0" 1.0 1.0 0.0 0 0 0 0)
  (bind _returnvalue (Utilities|Time|SetTimerbyEvent (delegate Custom|SacudirLocker) 0.05 true))
  (Variables|Locker|SetTimerTemblor _returnvalue)
  (Utilities|Time|SetTimerbyEvent (delegate Custom|DetenerTemblor) (Variables|Locker|GetDuracionTemblor)))

(event Custom|SacudirLocker
  (CallFunction|AplicarSacudida))

(event Custom|DetenerTemblor
  (Utilities|Time|ClearandInvalidateTimerbyHandle (Variables|Locker|GetTimerTemblor))
  (Transformation|SetRelativeRotation (Variables|Default|GetMeshLocker) (Variables|Locker|GetRotacionInicial) false false))

(event EventBeginPlay
  (bind _puertaobservada (Variables|Locker|GetPuertaObservada))
  (Variables|Locker|SetRotacionInicial (Variables|/Script/Engine.SceneComponent|GetRelativeRotation (Variables|Default|GetMeshLocker)))
  (Utilities|IsValid _puertaobservada
    (:Is%20Valid
      (EventDispatchers|BindEventtoOnInteractuado _puertaobservada (delegate Custom|AlAbrirsePuerta)))))

(fn ConstructionScript)

(fn AplicarSacudida
  (Transformation|SetRelativeRotation (Variables|Default|GetMeshLocker) (Math|Rotator|CombineRotators (Variables|Locker|GetRotacionInicial) (Math|Rotator|MakeRotator (Math|Random|RandomFloatinRange (* (Variables|Locker|GetIntensidad%20Temblor) -1.0) (Variables|Locker|GetIntensidad%20Temblor)) 0.0 (Math|Random|RandomFloatinRange (* (Variables|Locker|GetIntensidad%20Temblor) -1.0) (Variables|Locker|GetIntensidad%20Temblor)))) false false))